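; BP_FastNoise is an actor that builds a noise-driven height field out of instanced static meshes.
; On BeginPlay it creates a FastNoise object from a library function and loops over an X by Y grid.
; Each cell samples 2D noise at its index and adds a local-space instance, spaced by Span and raised by the noise value times Height.
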(event EventBeginPlay
  (bind _span (Variables|Default|GetSpan))
  (bind _returnvalue (Class|FastNoiseLibUtils|LibCreateFastNoiseObject self))
  (Variables|Default|SetFNO _returnvalue)
  (for _index (range 0 (- (Variables|Default|GetX) 1))
    (for _index_2 (range 0 (- (Variables|Default|GetY) 1))
      (bind _returnvalue_2 (Class|FastNoiseObject|GetNoiseValue2D (Variables|Default|GetFNO) _index _index_2))
      (Components|InstancedStaticMesh|AddInstance (Variables|Default|GetInstancedStaticMesh) (Math|Transform|MakeTransform (Math|Vector|MakeVector (* _index _span) (* _index_2 _span) (* _returnvalue_2 (Variables|Default|GetHeight)))) false))))

(fn ConstructionScript)