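; Advanced FastNoise demo actor that renders configurable noise to a render target and shows it on a plane with adjustable height displacement.
; On BeginPlay it creates a FastNoise object, applies a dynamic M_FN material to the plane and opens the WBP_ParamControl widget.
; Update events pass new noise parameters, refill RT_Example through a threaded fill and set the material's WPO value.
; Key 1 toggles between two threaded draw methods.
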(event Custom|BP_Update
  (params (CreateParams :type Noise%20Create%20Params%20Structure))
  (bind _fno (Variables|Default|GetFNO))
  (Class|FastNoiseObject|SetNoiseCreateParam _fno CreateParams)
  (Class|FastNoiseObject|FillDatatoRenderTargetThread _fno "/FastNoiseLite/RT_Example.RT_Example"))

(event Custom|BP_UpdateWPO
  (params (Value :type Float%20%28single-precision%29))
  (bind _mid (Variables|Default|GetMID)
    (:then
      (Rendering|Material|SetScalarParameterValue _mid "WPO" Value :!class /Script/Engine.MaterialInstanceDynamic))
    (:else)))

(event EventBeginPlay
  (bind _returnvalue (Game|GetPlayerController 0))
  (bind _returnvalue_2 (Class|FastNoiseLibUtils|LibCreateFastNoiseObject self))
  (Variables|Default|SetFNO _returnvalue_2)
  (bind _returnvalue_3 (Rendering|Material|CreateDynamicMaterialInstance "/FastNoiseLite/02/M_FN.M_FN" "None" "None" :!class /Script/Engine.KismetMaterialLibrary))
  (bind _output_get (Variables|Default|SetMID _returnvalue_3))
  (Rendering|Material|SetMaterial (Variables|Default|GetPlane) 0 _output_get)
  (bind _returnvalue_4 (UserInterface|CreateWidget "/FastNoiseLite/02/WBP_ParamControl.WBP_ParamControl_C" _returnvalue self))
  (UserInterface|Viewport|AddtoViewport _returnvalue_4 0)
  (Variables|/Script/Engine.PlayerController|SetbShowMouseCursor _returnvalue true)
  (Input|EnableInput _returnvalue))

(event Input|KeyboardEvents|1
  (params (Key :type Key%20Structure))
  (:Pressed
    (Utilities|FlowControl|FlipFlop
      (:A
        (bind _fno (Variables|Default|GetFNO)
          (:then
            (Class|FastNoiseObject|SetDrawThreadParam _fno "EMethod1" 1.0)
            (Development|PrintString "set to method 1"))
          (:else)))
      (:B
        (bind _fno_2 (Variables|Default|GetFNO)
          (:then
            (Class|FastNoiseObject|SetDrawThreadParam _fno_2 "EMethod2" 1.0)
            (Development|PrintString "set to method 2"))
          (:else))))))

(fn ConstructionScript)